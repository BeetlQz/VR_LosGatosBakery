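; VR stove knob actor that turns when grabbed and heats the stove top once fully rotated.
; Grabbing starts a looping timer for UpdateRotation, targeted at the motion controller rather than the knob, and dropping clears it.
; UpdateRotation derives clamped yaw from the controller's relative Z offset.
; Tick plays the Light timeline at maximum yaw, setting a fixed StoveTopHot value in a material parameter collection.
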(event OnGrabbed(GrabComponent)
  (params (Motion :type Motion%20Controller%20Component%20Object%20Reference))
  (bind _output_get (Variables|Default|SetMotion%20Controller Motion))
  (bind _returnvalue (Utilities|Time|SetTimerbyFunctionName _output_get "UpdateRotation" 0.02 true))
  (Variables|Default|SetTimer _returnvalue))

(event OnDropped(GrabComponent)
  (Utilities|Time|ClearandInvalidateTimerbyHandle (Variables|Default|GetTimer))
  (Variables|Default|SetMotion%20Controller 0))

(event EventBeginPlay)

(event Collision|EventActorBeginOverlap
  (params (OtherActor :type Actor%20Object%20Reference)))

(event EventTick
  (params (DeltaSeconds :type Float%20%28single-precision%29))
  (if (>= (.yaw (Variables|/Script/Engine.SceneComponent|GetRelativeRotation (Variables|Default|GetScene))) 9e+01)
    (Timeline|Light Play
      (:Update
        (Rendering|Material|SetScalarParameterValue "/Game/Materials/StoveStopParamCollection.StoveStopParamCollection" "StoveTopHot" 25.0 :!class /Script/Engine.KismetMaterialLibrary)))))

(fn ConstructionScript)

(fn UpdateRotation
  (bind _grabcomponent (Variables|Default|GetGrabComponent))
  (bind _scene (Variables|Default|GetScene))
  (bind _relativerotation (Variables|/Script/Engine.SceneComponent|GetRelativeRotation _scene))
  (Transformation|SetRelativeRotation _scene (Math|Rotator|MakeRotator (.roll _relativerotation) (.pitch _relativerotation) (Math|Float|Clamp(Float) (+ (.yaw _relativerotation) (.z (- (Variables|/Script/Engine.SceneComponent|GetRelativeLocation _grabcomponent) (.location (Math|Transform|MakeRelativeTransform (Transformation|GetWorldTransform (Variables|Default|GetMotion%20Controller)) (Transformation|GetWorldTransform _grabcomponent)))))) 0.0 9e+01)) false false))