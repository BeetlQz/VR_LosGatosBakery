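; BP_DMButton is a button that reacts to a VRPawn entering and leaving its overlap Box.
; BeginPlay stores the ControlButton's relative location as the rest position.
; Overlap events drive MoveComponentTo, intended to push the button down and return it.
; The stored Z, lowered by a fixed offset while pressed, feeds the target rotation's yaw rather than target location, despite the comments describing vertical movement.
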(event OnComponentBeginOverlap(Box)
  (params (OverlappedComponent :type Primitive%20Component%20Object%20Reference) (OtherActor :type Actor%20Object%20Reference) (OtherComp :type Primitive%20Component%20Object%20Reference) (OtherBodyIndex :type Integer) (bFromSweep :type Boolean) (SweepResult :type Hit%20Result%20Structure%20%28by%20ref%29))
  ;[0.15 0.15 0.15 0.5] On Player Overlap Push Button Down
  (Utilities|Casting|CastToVRPawn OtherActor)
  (Components|MoveComponentTo (Variables|Default|GetControlButton) "0, 0, 0" (Math|Rotator|MakeRotator 0.0 0.0 (- (.z (Variables|Default|GetButtonStartPosition)) 1e+01)) false false 0.2 false))

(event OnComponentEndOverlap(Box)
  (params (OverlappedComponent :type Primitive%20Component%20Object%20Reference) (OtherActor :type Actor%20Object%20Reference) (OtherComp :type Primitive%20Component%20Object%20Reference) (OtherBodyIndex :type Integer))
  ;[0.15 0.15 0.15 0.5] On Player End Overlap Button Returns to Start Position
  (Utilities|Casting|CastToVRPawn OtherActor)
  (Components|MoveComponentTo (Variables|Default|GetControlButton) "0, 0, 0" (Math|Rotator|MakeRotator 0.0 0.0 (.z (Variables|Default|GetButtonStartPosition))) false false 0.2 false))

(event EventBeginPlay
  ;[0.15 0.15 0.15 0.5] Set Button Start Location
  (Variables|Default|SetButtonStartPosition (Variables|/Script/Engine.SceneComponent|GetRelativeLocation (Variables|Default|GetControlButton))))

(fn ConstructionScript)