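; LowerCabinet is a cabinet Blueprint with a grab component, apparently meant as a VR hinged door that is still unfinished.
; Grabbing stores the motion controller and starts a looping UpdateRotation timer, targeted at the controller rather than the cabinet; dropping clears both.
; UpdateRotation only zeroes the Scene component's pitch and yaw, leaving the controller-driven, clamped yaw calculation unconnected.
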(event OnGrabbed(GrabComponent)
  (params (MotionController :type Motion%20Controller%20Component%20Object%20Reference))
  (bind _output_get (Variables|Default|SetMotion%20Controller MotionController))
  (bind _returnvalue (Utilities|Time|SetTimerbyFunctionName _output_get "UpdateRotation" 0.01 true))
  (Variables|Default|SetTimer _returnvalue))

(event OnDropped(GrabComponent)
  (Utilities|Time|ClearandInvalidateTimerbyHandle (Variables|Default|GetTimer))
  (Variables|Default|SetMotion%20Controller 0))

(fn ConstructionScript)

(fn UpdateRotation
  (bind _scene (Variables|Default|GetScene))
  (Transformation|SetRelativeRotation _scene (Math|Rotator|MakeRotator (.roll (Variables|/Script/Engine.SceneComponent|GetRelativeRotation _scene)) 0.0 0.0) false false))