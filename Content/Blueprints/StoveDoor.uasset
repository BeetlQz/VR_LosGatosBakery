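; StoveDoor is a stove door that swings open and shut when grabbed with a motion controller.
; Grabbing stores the controller and starts a fast looping timer for UpdateRotation, set with that controller as target object rather than the door; dropping clears both.
; UpdateRotation adds an X offset, derived from the controller's position relative to the grab component, to the Scene component's pitch, clamped between closed and 80 degrees.
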(event OnGrabbed(GrabComponent)
  (params (MotionController :type Motion%20Controller%20Component%20Object%20Reference))
  (bind _output_get (Variables|Default|SetMotion%20Controller MotionController))
  (bind _returnvalue (Utilities|Time|SetTimerbyFunctionName _output_get "UpdateRotation" 0.01 true))
  (Variables|Default|SetTimer _returnvalue))

(event OnDropped(GrabComponent)
  (Utilities|Time|ClearandInvalidateTimerbyHandle (Variables|Default|GetTimer))
  (Variables|Default|SetMotion%20Controller 0))

(fn ConstructionScript)

(fn UpdateRotation
  (bind _grabcomponent (Variables|Default|GetGrabComponent))
  (bind _scene (Variables|Default|GetScene))
  (bind _relativerotation (Variables|/Script/Engine.SceneComponent|GetRelativeRotation _scene))
  (Transformation|SetRelativeRotation _scene (Math|Rotator|MakeRotator (.roll _relativerotation) (Math|Float|Clamp(Float) (+ (.pitch _relativerotation) (.x (- (Variables|/Script/Engine.SceneComponent|GetRelativeLocation _grabcomponent) (.location (Math|Transform|MakeRelativeTransform (Transformation|GetWorldTransform (Variables|Default|GetMotion%20Controller)) (Transformation|GetWorldTransform _grabcomponent)))))) 0.0 8e+01) (.yaw _relativerotation)) false false))